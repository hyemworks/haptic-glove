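; BP_Sphere is a touchable sphere actor that reports contact with a BP_UE4Duino actor to an Arduino.
; On overlap begin, it sets the "touch" field in that actor's output JSON to true, prints it to the Arduino and on screen, then calls Grip.
; On overlap end, it calls InitializeOUTPUTJSON on that actor, without sending anything to the Arduino itself.
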(event EventBeginPlay)

(event EventTick
  (params (DeltaSeconds :type Float%20%28single-precision%29)))

(event Collision|EventActorBeginOverlap
  (params (OtherActor :type Actor%20Object%20Reference))
  ;[1 1 1] Touch
  (bind _asbp_ue4duino (Utilities|Casting|CastToBP_UE4Duino OtherActor))
  (Class|BlueprintJsonLibrary|JsonSetField (Variables|/Game/_hmyang/Blueprints/BP_UE4Duino.BP_UE4Duino_C|GetOUTPUT%20JSON _asbp_ue4duino) "touch" (Class|BlueprintJsonLibrary|JsonMakeBool true))
  (Class|Serial|Print (Variables|/Game/_hmyang/Blueprints/BP_UE4Duino.BP_UE4Duino_C|GetArduino _asbp_ue4duino) (Class|BlueprintJsonLibrary|ToString(JsonObject) (Variables|/Game/_hmyang/Blueprints/BP_UE4Duino.BP_UE4Duino_C|GetOUTPUT%20JSON _asbp_ue4duino)))
  (Development|PrintString (Class|BlueprintJsonLibrary|ToString(JsonObject) (Variables|/Game/_hmyang/Blueprints/BP_UE4Duino.BP_UE4Duino_C|GetOUTPUT%20JSON _asbp_ue4duino)) true true "(R=0.000000,G=0.000000,B=0.000000,A=1.000000)" 5.0)
  (Default|Grip _asbp_ue4duino))

(event Collision|EventActorEndOverlap
  (params (OtherActor :type Actor%20Object%20Reference))
  ;[1 1 1] End Touch
  (bind _asbp_ue4duino (Utilities|Casting|CastToBP_UE4Duino OtherActor))
  (Default|InitializeOUTPUTJSON _asbp_ue4duino))

(fn ConstructionScript)